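; Car pickup actor that destroys itself when the BP_MyCarProjectPawn overlaps it, with no reward logic in this graph.
; Each Tick moves the static mesh vertically by UpDown and adds pitch, feeding world location and rotation into a relative-transform setter.
; A one-second Delay on Tick flips UpDown's sign to alternate the bob direction, with movement independent of delta time.
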(event `self.ReceiveActorBeginOverlap`
  (params (OtherActor :type "Actor Object Reference"))
  (cast `/Game/Blueprints/BP_MyCarProjectPawn` OtherActor)
  (`self.K2_DestroyActor`))

(event `self.ReceiveTick`
  (params (DeltaSeconds :type "Float (single-precision)"))
  (`SceneComponent.K2_SetRelativeLocationAndRotation` (`self.StaticMeshComponent`) (`KismetMathLibrary.MakeVector` (.x (`SceneComponent.K2_GetComponentLocation` (`self.StaticMeshComponent`))) (.y (`SceneComponent.K2_GetComponentLocation` (`self.StaticMeshComponent`))) (+ (.z (`SceneComponent.K2_GetComponentLocation` (`self.StaticMeshComponent`))) (`self.Up_Down`))) (`KismetMathLibrary.MakeRotator` (.roll (`SceneComponent.K2_GetComponentRotation` (`self.StaticMeshComponent`))) (+ (.pitch (`SceneComponent.K2_GetComponentRotation` (`self.StaticMeshComponent`))) 1.0) (.yaw (`SceneComponent.K2_GetComponentRotation` (`self.StaticMeshComponent`)))) false false)
  (`KismetSystemLibrary.Delay` 1.0)
  (if (== (`self.Up_Down`) 0.5)
    (set `self.Up_Down` -0.5)
    (else
      (set `self.Up_Down` 0.5))))

(fn `UserConstructionScript`)