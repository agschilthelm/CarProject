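; Game mode that respawns the player's car pawn after it is destroyed.
; On BeginPlay it binds to the player pawn's OnDestroyed event.
; When that fires, it waits briefly, spawns a new BP_MyCarProjectPawn at the stored Spawn transform and possesses it with the player controller.
; It then calls Respawn to rebind the destroy event on the new pawn, so the cycle repeats.
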(event `Respawn`
  (bind _asbp_my_car_project_pawn (cast `/Game/Blueprints/BP_MyCarProjectPawn` (`GameplayStatics.GetPlayerPawn` 0) :!label _label))
  (add `Actor.OnDestroyed` _asbp_my_car_project_pawn (delegate `OnDestroyed_Event`)))

(event `self.ReceiveBeginPlay`
  (goto _label))

(event `OnDestroyed_Event`
  (params (DestroyedActor :type "Actor Object Reference"))
  (`KismetSystemLibrary.Delay` 2.0)
  (bind _returnvalue (`|SpawnActorFromClass` "/Game/Blueprints/BP_MyCarProjectPawn.BP_MyCarProjectPawn_C" (`self.Spawn`) "AdjustIfPossibleButAlwaysSpawn" "OverrideRootScale" null null))
  (`Controller.Possess` (`GameplayStatics.GetPlayerController` 0) _returnvalue)
  (`self.Respawn`))

(fn `UserConstructionScript`)