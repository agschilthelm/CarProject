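; BP_MyCarProjectPawn is a car pawn with health that can be damaged and destroyed.
; On BeginPlay it creates and stores a HUD widget and adds it to the viewport.
; Projectile hits on the mesh and a Hurt input action each reduce Health, print it, and destroy the pawn at zero or below.
; A projectile that hits the mesh is destroyed as well.
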(event `self.ReceiveBeginPlay`
  (bind _returnvalue (`|CreateWidget` "/Game/Blueprints/HUD.HUD_C"))
  (bind _output_get (set `self.HUD Reference` _returnvalue))
  (`UserWidget.AddToViewport` _output_get 0))

(event `InputAction|Hurt`
  (params (Key :type "Key Structure"))
  (:`Pressed`
    (bind _output_get (set `self.Health` (- (`self.Health`) 50)))
    (`KismetSystemLibrary.PrintString` (`KismetStringLibrary.Conv_IntToString` _output_get))
    (if (<= (`self.Health`) 0)
      (`self.K2_DestroyActor`))))

(event `self.Mesh.OnComponentHit`
  (params (HitComponent :type "PrimitiveComponent Object Reference") (OtherActor :type "Actor Object Reference") (OtherComp :type "PrimitiveComponent Object Reference") (NormalImpulse :type "Vector Structure") (Hit :type "HitResult Structure (by ref)"))
  (bind _asbp_aprojectile (cast `/Game/Blueprints/BP_AProjectile` OtherActor))
  (bind _output_get (set `self.Health` (- (`self.Health`) 25)))
  (`KismetSystemLibrary.PrintString` (`KismetStringLibrary.Conv_IntToString` _output_get))
  (if (<= (`self.Health`) 0)
    (`self.K2_DestroyActor`)
    (`self.K2_DestroyActor` _asbp_aprojectile)
    (else
      (`self.K2_DestroyActor` _asbp_aprojectile))))

(fn `UserConstructionScript`)